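; BP_Door is a two-sided door that moves the player between adjacent rooms in a Metroidvania-style game.
; On BeginPlay it finds each side's room camera from the first camera actor overlapping that side's spawn location component.
; Entering either trigger flags the character as moving through a door and gives it the opposite side's spawn position and camera.
; It then calls RoomTransition on the game mode.
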(event OnComponentBeginOverlap(DoorTrigger(Right))
  (params (OverlappedComponent :type Primitive%20Component%20Object%20Reference) (OtherActor :type Actor%20Object%20Reference) (OtherComp :type Primitive%20Component%20Object%20Reference) (OtherBodyIndex :type Integer) (bFromSweep :type Boolean) (SweepResult :type Hit%20Result%20Structure%20%28by%20ref%29))
  (bind _asbp_metroidvania_character (Utilities|Casting|CastToBP_MetroidvaniaCharacter OtherActor))
  (Variables|/Game/Source/Blueprints/BP_MetroidvaniaCharacter.BP_MetroidvaniaCharacter_C|SetIsMovingThroughDoor _asbp_metroidvania_character true)
  (Variables|/Game/Source/Blueprints/BP_MetroidvaniaCharacter.BP_MetroidvaniaCharacter_C|SetNewSpawnPosition _asbp_metroidvania_character (Transformation|GetWorldLocation (Variables|Default|GetLeftSpawnLocation)))
  (Variables|/Game/Source/Blueprints/BP_MetroidvaniaCharacter.BP_MetroidvaniaCharacter_C|SetCurrentCamera _asbp_metroidvania_character (Variables|Default|GetLeftCamera))
  (bind _asbp_metroidvania_game_mode (Utilities|Casting|CastToBP_MetroidvaniaGameMode (Game|GetGameMode)))
  (Default|RoomTransition _asbp_metroidvania_game_mode))

(event OnComponentBeginOverlap(DoorTrigger(Left))
  (params (OverlappedComponent :type Primitive%20Component%20Object%20Reference) (OtherActor :type Actor%20Object%20Reference) (OtherComp :type Primitive%20Component%20Object%20Reference) (OtherBodyIndex :type Integer) (bFromSweep :type Boolean) (SweepResult :type Hit%20Result%20Structure%20%28by%20ref%29))
  (bind _asbp_metroidvania_character (Utilities|Casting|CastToBP_MetroidvaniaCharacter OtherActor))
  (Variables|/Game/Source/Blueprints/BP_MetroidvaniaCharacter.BP_MetroidvaniaCharacter_C|SetIsMovingThroughDoor _asbp_metroidvania_character true)
  (Variables|/Game/Source/Blueprints/BP_MetroidvaniaCharacter.BP_MetroidvaniaCharacter_C|SetNewSpawnPosition _asbp_metroidvania_character (Transformation|GetWorldLocation (Variables|Default|GetRightSpawnLocation)))
  (Variables|/Game/Source/Blueprints/BP_MetroidvaniaCharacter.BP_MetroidvaniaCharacter_C|SetCurrentCamera _asbp_metroidvania_character (Variables|Default|GetRightCamera))
  (bind _asbp_metroidvania_game_mode (Utilities|Casting|CastToBP_MetroidvaniaGameMode (Game|GetGameMode)))
  (Default|RoomTransition _asbp_metroidvania_game_mode))

(event EventBeginPlay
  (bind _asbp_metroidvania_camera (Utilities|Casting|CastToBP_MetroidvaniaCamera (Utilities|Array|Get(acopy) (Collision|GetOverlappingActors (Variables|Default|GetRightSpawnLocation) "/Game/Source/Blueprints/BP_MetroidvaniaCamera.BP_MetroidvaniaCamera_C" :!class /Script/Engine.PrimitiveComponent))))
  (Variables|Default|SetRightCamera _asbp_metroidvania_camera)
  (bind _asbp_metroidvania_camera_2 (Utilities|Casting|CastToBP_MetroidvaniaCamera (Utilities|Array|Get(acopy) (Collision|GetOverlappingActors (Variables|Default|GetLeftSpawnLocation) "/Game/Source/Blueprints/BP_MetroidvaniaCamera.BP_MetroidvaniaCamera_C" :!class /Script/Engine.PrimitiveComponent))))
  (Variables|Default|SetLeftCamera _asbp_metroidvania_camera_2))

(fn ConstructionScript)