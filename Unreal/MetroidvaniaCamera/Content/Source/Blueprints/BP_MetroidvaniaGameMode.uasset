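; Game mode for a metroidvania that runs the door transition between rooms through its RoomTransition event.
; It flags and hides the player, then a timeline drives a shared Material Parameter Collection opacity for the fade.
; It then teleports the player to their stored spawn position and blends to their current camera.
; After the blend, it clears the flag, reverses the fade and reveals the player.
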(event Custom|Room%20Transition
  (bind _asbp_metroidvania_character (Utilities|Casting|CastToBP_MetroidvaniaCharacter (Game|Player|GetPlayerPawn 0)))
  (Variables|/Game/Source/Blueprints/BP_MetroidvaniaCharacter.BP_MetroidvaniaCharacter_C|SetIsMovingThroughDoor _asbp_metroidvania_character true)
  (Rendering|SetActorHiddenInGame _asbp_metroidvania_character true)
  (bind _opacity (Timeline|Sprite%20Fadeout%20Timeline PlayFromStart)
    (:Update
      (Rendering|Material|SetScalarParameterValue "/Game/Source/Materials/MetroidvaniaParamCollection.MetroidvaniaParamCollection" "Opacity" (Math|Float|Lerp 0.0 1.0 _opacity) :!class /Script/Engine.KismetMaterialLibrary))
    (:On%20Complete
      (Transformation|Teleport _asbp_metroidvania_character (Variables|/Game/Source/Blueprints/BP_MetroidvaniaCharacter.BP_MetroidvaniaCharacter_C|GetNewSpawnPosition _asbp_metroidvania_character) "0,0.000000, 0")
      (Game|Player|SetViewTargetwithBlend (Game|GetPlayerController 0) (Variables|/Game/Source/Blueprints/BP_MetroidvaniaCharacter.BP_MetroidvaniaCharacter_C|GetCurrentCamera _asbp_metroidvania_character) 0.75 "VTBlend_EaseInOut" 2.0 false)
      (Utilities|FlowControl|Delay 0.75)
      (Variables|/Game/Source/Blueprints/BP_MetroidvaniaCharacter.BP_MetroidvaniaCharacter_C|SetIsMovingThroughDoor _asbp_metroidvania_character false)
      (bind _opacity_2 (Timeline|Sprite%20Fadein%20Timeline Play)
        (:Update
          (Rendering|Material|SetScalarParameterValue "/Game/Source/Materials/MetroidvaniaParamCollection.MetroidvaniaParamCollection" "Opacity" (Math|Float|Lerp 1.0 0.0 _opacity_2) :!class /Script/Engine.KismetMaterialLibrary))
        (:On%20Complete
          (Rendering|SetActorHiddenInGame _asbp_metroidvania_character false))))))

(event EventBeginPlay)

(event EventTick
  (params (DeltaSeconds :type Float%20%28single-precision%29)))

(fn ConstructionScript)