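; BP_MetroidvaniaCharacter is a side-scrolling flipbook character that runs and jumps.
; MoveRight input moves it along world X and flips controller yaw to face the travel direction.
; Jump input triggers the Jumping state, switching to Falling after a short delay if airborne, while Tick picks Run or Idle from velocity when not falling.
; SetAnimationState stores the state and selects the matching Sprite flipbook.
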(event EventTick
  (params (DeltaSeconds :type Float%20%28single-precision%29))
  (if (not (AI|Components|NavMovement|IsFalling (Variables|Character|GetCharacterMovement)))
    (CallFunction|SetAnimationState (select (> (Math|Vector|VectorLength (Transformation|GetVelocity)) 0.0) "NewEnumerator1" "NewEnumerator0"))))

(event Input|ActionEvents|InputActionJump
  (params (Key :type Key%20Structure :default "None"))
  ;[0 0 0] Jumping
  (:Pressed
    (Character|Jump)
    (if (Character|CanJump)
      (CallFunction|SetAnimationState "NewEnumerator2")
      (Utilities|FlowControl|Delay 0.2)
      (if (AI|Components|NavMovement|IsFalling (Variables|Character|GetCharacterMovement))
        (CallFunction|SetAnimationState "NewEnumerator3"))))
  (:Released
    (Character|StopJumping)))

(event Input|AxisEvents|InputAxisMoveRight
  (params (AxisValue :type Float%20%28single-precision%29))
  (bind _returnvalue (Pawn|GetController))
  (Math|Float|CompareFloat AxisValue 0.0
    (:>
      (Variables|Default|SetIsMovingRight true))
    (:<
      (Variables|Default|SetIsMovingRight false)))
  (Pawn|Input|AddMovementInput "1.000000, 0, 0" AxisValue false)
  (if (Variables|Default|GetIsMovingRight)
    (Pawn|SetControlRotation _returnvalue (Math|Rotator|MakeRotator 0.0 0.0 0.0))
    (else
      (Pawn|SetControlRotation _returnvalue (Math|Rotator|MakeRotator 0.0 0.0 1.8e+02)))))

(fn ConstructionScript)

(fn SetAnimationState
  (params (Anim%20State :type AnimationStates%20Enum :default "NewEnumerator0"))
  (Variables|Default|SetCurrentAnimationState Anim%20State)
  (Sprite|SetFlipbook (Variables|Default|GetSprite) (Utilities|Select :Index (Variables|Default|GetCurrentAnimationState) :NewEnumerator0 (Variables|Default|GetIdle) :NewEnumerator1 (Variables|Default|GetRun) :NewEnumerator2 (Variables|Default|GetJumping) :NewEnumerator3 (Variables|Default|GetFalling)))
  (return))